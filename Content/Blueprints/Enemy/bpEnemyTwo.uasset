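; Enemy Blueprint that repeatedly fires pairs of projectiles, extending the BeginPlay, Tick and construction logic of its parent class.
; Tick feeds a Delay of FireRate, which throttles firing because retriggers are ignored while it is pending.
; Each volley spawns two BpProjectileEnemy actors at the Top and Button component transforms, with fixed damage, scale and negative-Y speed.
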(event EventBeginPlay
  (|CallParentFunction))

(event EventTick
  (params (DeltaSeconds :type Float%20%28single-precision%29))
  (|CallParentFunction DeltaSeconds)
  (Utilities|FlowControl|Delay (Variables|Default|GetFireRate))
  (Game|SpawnActorfromClass "/Game/Blueprints/Projectiles/bpProjectileEnemy.bpProjectileEnemy_C" (Transformation|GetWorldTransform (Variables|Default|GetTop)) "Undefined" 0 2e+01 "0.000000,-2200.000000,0.000000" "2.500000,1.000000,1.000000" 0) ; Spawn Actor from class
  (Game|SpawnActorfromClass "/Game/Blueprints/Projectiles/bpProjectileEnemy.bpProjectileEnemy_C" (Transformation|GetWorldTransform (Variables|Default|GetButton)) "Undefined" 0 2e+01 "0.000000,-2200.000000,0.000000" "2.500000,1.000000,1.000000" 0) ; Spawn Actor from class
)

(fn ConstructionScript
  (|CallParentFunction))