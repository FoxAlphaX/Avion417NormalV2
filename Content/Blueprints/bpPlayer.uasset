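; Player ship Blueprint for a shooter, with a timeline spawn fly-in and roll that enables movement when finished.
; Tick eases vertical and horizontal input into swept movement, pitches the mesh, and runs cooldown timers behind input-driven Gates for primary and rocket fire.
; Primary fire spawns projectiles at random height offsets, while power-up and rocket volleys spawn BpPlayer copies.
; Damage sets health to clamped damage minus health; zero flags PlayerDead on bpGameMode and destroys the actor.
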(event Custom|FireRateControl
  (bind _projectilespawn (Variables|Default|GetProjectileSpawn))
  ;[1 1 1] Proyectiles
  (Utilities|FlowControl|Sequence
    (:then_0
      ;;[1 1 1] Cooldown de bala
      (Variables|Float|SetPrimariFireRate (- (Variables|Float|GetPrimariFireRate) (Variables|Float|GetDeltaSeconds)))
      (if (<= (Variables|Float|GetPrimariFireRate) 0.0)
        (Utilities|FlowControl|Gate true
          (:Exit
            (Variables|Float|SetPrimariFireRate (Variables|Float|GetPrimaryFireRateBase))
            (if (not (Variables|Default|GetbHasPower))
              (CallFunction|PrimaryFire _projectilespawn) ; Location donde aparecera la bala
              (else
                (CallFunction|PowerUpfire (Variables|Default|GetPower%20Shot%20Count) _projectilespawn)))))))
    (:then_1
      ;;[1 1 1] Cooldown de bala
      (Variables|Float|SetRocektyFireRate (- (Variables|Float|GetRocektyFireRate) (Variables|Float|GetDeltaSeconds)))
      (if (<= (Variables|Float|GetRocektyFireRate) 0.0)
        (Utilities|FlowControl|Gate true
          (:Exit
            (Variables|Float|SetRocektyFireRate (Variables|Float|GetRocektyFireRate))
            (if (Variables|Default|GetbHasRocket)
              (CallFunction|RocketFire (Variables|Default|GetRocketShoot%20count) _projectilespawn))))))))

(event EventBeginPlay
  ;[1 1 1] Spawn Animation
  (Variables|Float|SetHealth (Variables|Float|GetMaxHealth))
  (Variables|Float|SetPitch (.Pitch (Math|Rotator|BreakRotator (Variables|/Script/Engine.SceneComponent|GetRelativeRotation (Variables|Default|GetPlayerMesh)))))
  (Variables|Default|SetSpawnrRotation (Transformation|GetWorldRotation (Variables|Default|GetPlayerMesh)))
  (Variables|Default|SetSpawnLocation (Transformation|GetActorLocation))
  (bind _spawn (Timeline|TimelineSpawnAnimation Play)
    (:Update
      (Transformation|SetActorLocation (Math|Vector|Lerp(Vector) (Variables|Default|GetSpawnLocation) (+ (Variables|Default|GetSpawnLocation) "0,1000.000000, 0") _spawn) false false)
      (Transformation|SetRelativeRotation (Variables|Default|GetPlayerMesh) (Math|Rotator|Lerp(Rotator) (Variables|Default|GetSpawnrRotation) (Math|Rotator|MakeRotator 0.0 (+ (Variables|Default|GetAnimationPitch) (Variables|Float|GetPitch)) 0.0) _spawn) false false))
    (:Finished
      (Variables|Default|SetbMovementEnabled true) ; se puso despues este cuadrote para decirle a tock que ay se puede mover
    )))

(event EventTick
  (params (DeltaSeconds :type Float%20%28single-precision%29))
  ;[1 1 1] Movement
  (Variables|Float|SetDeltaSeconds DeltaSeconds)
  (if (Variables|Default|GetbMovementEnabled)
    (CallFunction|FireRateControl)
    (Utilities|FlowControl|Sequence
      (:then_0
        (bind _returndirection (CallFunction|GetDirection (Variables|Float|GetVertSpeed) (Input|AxisValues|GetMoveUp))) ; Doble Clic aqui para ver que hay dentro de la Funcion, se podria poner lo de dentro aqui pero seria muchos nodos a la vista y mejor crear estas funciones
        (Variables|Float|SetVertSpeed _returndirection))
      (:then_1
        (bind _returndirection_2 (CallFunction|GetDirection (Variables|Float|GetHorizSpeed) (Input|AxisValues|GetMoveRight)))
        (Variables|Float|SetHorizSpeed _returndirection_2))
      (:then_2
        (Transformation|SetActorLocation (+ (Transformation|GetActorLocation) (Math|Vector|MakeVector 0.0 0.0 (Variables|Float|GetVertSpeed))) true false) ; Mueve en Vertical
        (Transformation|SetActorLocation (+ (Transformation|GetActorLocation) (Math|Vector|MakeVector 0.0 (Variables|Float|GetHorizSpeed) 0.0)) true false) ; Mueve en Horizontal
        (if (> (Variables|Float|GetHealth) 0.0) ; Rotal al Mover Vertical
          (Transformation|SetRelativeRotation (Variables|Default|GetPlayerMesh) (Math|Interpolation|RInterpTo (Transformation|GetActorRotation) (Math|Rotator|MakeRotator 0.0 (Variables|Float|GetVertSpeed) 0.0) (Variables|Float|GetDeltaSeconds) 8e+01) false false) ; Para que gire la nave al subir o bajar
        )))))

(event Game|Damage|EventAnyDamage
  (params (Damage :type Float%20%28single-precision%29) (DamageType :type Damage%20Type%20Object%20Reference) (InstigatedBy :type Controller%20Object%20Reference) (DamageCauser :type Actor%20Object%20Reference))
  ;[1 1 1] Player Dead
  (Variables|Float|SetHealth (Math|Float|Clamp(Float) (- Damage (Variables|Float|GetHealth)) 0.0 (Variables|Float|GetMaxHealth)))
  (if (<= (Variables|Float|GetHealth) 0.0)
    (bind _asbp_game_mode (Utilities|Casting|CastTobpGameMode (Game|GetGameMode)))
    (Variables|/Game/Blueprints/BpGameMode.bpGameMode_C|SetbPlayerDead _asbp_game_mode true)
    (Actor|DestroyActor)))

(event Input|ActionEvents|InputActionPrimaryFire
  (params (Key :type Key%20Structure))
  (bind _projectilespawn (Variables|Default|GetProjectileSpawn))
  ;[1 1 1] Proyectiles
  ;;[1 1 1] Cooldown de bala
  (:Pressed
    (Utilities|FlowControl|Gate true) ; enters at Open
  )
  (:Released
    (Utilities|FlowControl|Gate true) ; enters at Close
  ))

(event Input|ActionEvents|InputActionRocketFire
  (params (Key :type Key%20Structure))
  ;[1 1 1] Proyectiles
  ;;[1 1 1] Cooldown de bala
  (:Pressed
    (Utilities|FlowControl|Gate true) ; enters at Open
  )
  (:Released
    (Utilities|FlowControl|Gate true) ; enters at Close
  ))

(fn ConstructionScript)

(fn GetDirection
  (params (Speed :type Float%20%28single-precision%29) (Direction :type Float%20%28single-precision%29))
  (bind _output_get (Variables|Float|SetCurrentSpeed (Math|Interpolation|FInterpTo Speed (* (* Direction (Variables|Float|GetMoventSpeed)) (Variables|Float|GetDeltaSeconds)) (Variables|Float|GetDeltaSeconds) 4.0))) ; se podia ir directo de FlnterpTo pero se agrego SetCurrentSpeed
  (return _output_get))

(fn PrimaryFire
  (params (spawnLocarion :type Scene%20Component%20Object%20Reference))
  (bind _returnvalue (Transformation|GetWorldTransform spawnLocarion))
  (bind (_location _rotation) (Math|Transform|BreakTransform _returnvalue))
  (Game|SpawnActorfromClass "/Game/Blueprints/Projectiles/bpProjectilePlayerPrimary.bpProjectilePlayerPrimary_C" (Math|Transform|MakeTransform (Math|Vector|MakeVector (.x _location) (.y _location) (+ (.z _location) (Math|Random|RandomFloatinRange -7e+01 7e+01))) _rotation) "AlwaysSpawn" 0 0) ; SpawnActor from class, aqui llega el BP del proyectil primario
)

(fn PowerUpfire
  (params (NumersOfShots :type Integer) (SpaenLocation :type Scene%20Component%20Object%20Reference))
  (bind _returnvalue (Transformation|GetWorldTransform SpaenLocation))
  (bind _location (Math|Transform|BreakTransform _returnvalue))
  (LocalVariables|SetOffset (/ NumersOfShots -2)) ; Offset: Por ejemplo, dado un array de caracteres "A" que contenga "abcdef", se puede decir que el elemento que contiene el caracter "'d'" tiene un offset de 4 desde el comienzo de A.
  (for _index (range 0 NumersOfShots)
    (Development|PrintString (Utilities|String|ToString(Float) (+ (.z _location) (* (Math|Conversions|ToFloat(Integer) (LocalVariables|GetOffset)) 5.0))) true true "(R=0.000000,G=0.660000,B=1.000000,A=1.000000)" 9e+02)
    (Game|SpawnActorfromClass "bpPlayer_C" (Math|Transform|MakeTransform (Math|Vector|MakeVector (.x _location) (.y _location) (+ (.z _location) (* (Math|Conversions|ToFloat(Integer) (LocalVariables|GetOffset)) 5.0))) (Math|Rotator|MakeRotator (* (Math|Conversions|ToFloat(Integer) (LocalVariables|GetOffset)) 5.0) 0.0 0.0)) "AlwaysSpawn" 0 0)
    (LocalVariables|SetOffset (+ (LocalVariables|GetOffset) 1))))

(fn RocketFire
  (params (NumberOfShoot :type Integer) (SpawnLocation :type Scene%20Component%20Object%20Reference))
  (bind _returnvalue (Transformation|GetWorldTransform SpawnLocation))
  (bind _location (Math|Transform|BreakTransform _returnvalue))
  (LocalVariables|SetOffset (/ (+ NumberOfShoot 1) -1))
  (for _index (range 0 NumberOfShoot)
    (Game|SpawnActorfromClass "bpPlayer_C" (Math|Transform|MakeTransform (Math|Vector|MakeVector (.x _location) (.y _location) (+ (.z _location) (* (Math|Conversions|ToFloat(Integer) (LocalVariables|GetOffset)) 5.0))) (Math|Rotator|MakeRotator (* (Math|Conversions|ToFloat(Integer) (LocalVariables|GetOffset)) 5.0) 0.0 0.0)) "AlwaysSpawn" 0 0)
    (LocalVariables|SetOffset (+ (LocalVariables|GetOffset) 4))))