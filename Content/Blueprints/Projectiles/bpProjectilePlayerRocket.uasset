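; Player rocket projectile Blueprint with homing logic that currently targets bpPlayer, apparently as a stand-in for an enemy reference.
; A homing box overlap stores the first player it detects while no valid target is held.
; Each Tick lerps ProjectileMovement velocity toward the normalized target direction plus a speed variable (added, not multiplied).
; The lerp alpha is zero, so the homing leaves velocity unchanged as written.
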(event OnComponentBeginOverlap(HomingBoxCajaDeReferencia)
  (params (OverlappedComponent :type Primitive%20Component%20Object%20Reference) (OtherActor :type Actor%20Object%20Reference) (OtherComp :type Primitive%20Component%20Object%20Reference) (OtherBodyIndex :type Integer) (bFromSweep :type Boolean) (SweepResult :type Hit%20Result%20Structure%20%28by%20ref%29))
  ;[1 1 1] Relace whit enemy reference
  (bind _asbp_player (Utilities|Casting|CastTobpPlayer OtherActor))
  (Utilities|IsValid (Variables|Default|GetTempVar)
    (:Is%20Not%20Valid
      (Variables|Default|SetTempVar _asbp_player))))

(event EventTick
  (params (DeltaSeconds :type Float%20%28single-precision%29))
  (Utilities|IsValid (Variables|Default|GetTempVar)
    (:Is%20Valid
      (Variables|/Script/Engine.MovementComponent|SetVelocity (Variables|Default|GetProjectileMovement) (Math|Vector|Lerp(Vector) (Variables|/Script/Engine.MovementComponent|GetVelocity (Variables|Default|GetProjectileMovement)) (+ (Math|Vector|Normalize (- (Transformation|GetActorLocation (Variables|Default|GetTempVar)) (Transformation|GetActorLocation))) (Variables|Default|GetIncresedSpeed)) 0.0)))))

(fn ConstructionScript
  (|CallParentFunction))