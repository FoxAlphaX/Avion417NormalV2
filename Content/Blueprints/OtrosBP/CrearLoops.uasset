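; CrearLoops is a Blueprint that sketches a hand-built counting loop, with no event driving it.
; A temporary counter starts at zero, and a switch on the comparison operator selects the bound check.
; Less-than checks increment the counter and greater-than checks decrement it, each looping back through a Sequence node.
; The loop body and compared bound are unconnected, and the Construction Script is empty.
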(fn ConstructionScript)